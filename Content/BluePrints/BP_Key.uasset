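; BP_Key is a pickup key actor that grants the player one of two keys.
; A trigger overlap shows the Textkey prompt while the player character is inside and hides it on exit or at game start.
; On Interact it casts the player to BP_ThirdPersonCharacter and, based on IsKey1 or IsKey2, sets the matching HasKey flag if unset, then destroys itself.
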(event OnComponentBeginOverlap(Trigger)
  (params (OverlappedComponent :type Primitive%20Component%20Object%20Reference) (OtherActor :type Actor%20Object%20Reference) (OtherComp :type Primitive%20Component%20Object%20Reference) (OtherBodyIndex :type Integer) (bFromSweep :type Boolean) (SweepResult :type Hit%20Result%20Structure%20%28by%20ref%29))
  ;[0.3923 1 0.294] Accendo e spengo Text quando entra ed esce il caracter dal trigger
  (if (== OtherActor (Game|GetPlayerCharacter 0))
    (Development|SetHiddeninGame (Variables|Default|GetTextkey) false false)))

(event OnComponentEndOverlap(Trigger)
  (params (OverlappedComponent :type Primitive%20Component%20Object%20Reference) (OtherActor :type Actor%20Object%20Reference) (OtherComp :type Primitive%20Component%20Object%20Reference) (OtherBodyIndex :type Integer))
  ;[0.3923 1 0.294] Accendo e spengo Text quando entra ed esce il caracter dal trigger
  (if (== (Game|GetPlayerCharacter 0) OtherActor)
    (Development|SetHiddeninGame (Variables|Default|GetTextkey) true false)))

(event EventBeginPlay
  ;[0.276 0.2305 0.07059] Inzio partita spegne test interazione
  (Development|SetHiddeninGame (Variables|Default|GetTextkey) true false))

(event EventInteract
  ;[1 1 1] Per fare scopararire la chiave dopo interazione
  (bind _asbp_third_person_character (Utilities|Casting|CastToBP_ThirdPersonCharacter (Game|GetPlayerCharacter 0)))
  (if (Variables|Default|GetisKey1)
    (if (not (Variables|/Game/ThirdPerson/Blueprints/BP_ThirdPersonCharacter.BP_ThirdPersonCharacter_C|GethasKey1 _asbp_third_person_character))
      (Variables|/Game/ThirdPerson/Blueprints/BP_ThirdPersonCharacter.BP_ThirdPersonCharacter_C|SethasKey1 _asbp_third_person_character true)
      (Actor|DestroyActor :!label _label))
    (elif (Variables|Default|GetisKey2)
      (if (not (Variables|/Game/ThirdPerson/Blueprints/BP_ThirdPersonCharacter.BP_ThirdPersonCharacter_C|GethasKey2 _asbp_third_person_character))
        (Variables|/Game/ThirdPerson/Blueprints/BP_ThirdPersonCharacter.BP_ThirdPersonCharacter_C|SethasKey2 _asbp_third_person_character true)
        (goto _label)))))

(fn ConstructionScript)