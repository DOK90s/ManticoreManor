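; BP_Door is an interactable hinged door that swings away in either direction and closes automatically.
; Front and back box triggers track the player, and Interact opens a closed door from that side if its CanOpen flag allows.
; Separate timelines rotate the pivot 90 degrees in opposite yaw directions.
; Leaving either trigger while open reverses that side's timeline, regardless of which side opened it.
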(event OnComponentBeginOverlap(BoxCollider_front)
  (params (OverlappedComponent :type Primitive%20Component%20Object%20Reference) (OtherActor :type Actor%20Object%20Reference) (OtherComp :type Primitive%20Component%20Object%20Reference) (OtherBodyIndex :type Integer) (bFromSweep :type Boolean) (SweepResult :type Hit%20Result%20Structure%20%28by%20ref%29))
  ;[0.3033 0.3213 1] DoorPlayerDetectionFront
  (if (== OtherActor (Game|GetPlayerCharacter 0))
    (Variables|Default|SetPlayerFront true)))

(event OnComponentEndOverlap(BoxCollider_front)
  (params (OverlappedComponent :type Primitive%20Component%20Object%20Reference) (OtherActor :type Actor%20Object%20Reference) (OtherComp :type Primitive%20Component%20Object%20Reference) (OtherBodyIndex :type Integer))
  ;[0.3033 0.3213 1] DoorPlayerDetectionFront
  (if (== (Game|GetPlayerCharacter 0) OtherActor)
    (Variables|Default|SetPlayerFront false)
    (if (not (Variables|Default|GetDoorClosed))
      (CallFunction|ChiusuraFront))))

(event OnComponentBeginOverlap(BoxCollider_back)
  (params (OverlappedComponent :type Primitive%20Component%20Object%20Reference) (OtherActor :type Actor%20Object%20Reference) (OtherComp :type Primitive%20Component%20Object%20Reference) (OtherBodyIndex :type Integer) (bFromSweep :type Boolean) (SweepResult :type Hit%20Result%20Structure%20%28by%20ref%29))
  ;[0.3326 0.3792 1] DoorPlayerDetectionBack
  (if (== (Game|GetPlayerCharacter 0) OtherActor)
    (Variables|Default|SetPlayerBack true)))

(event OnComponentEndOverlap(BoxCollider_back)
  (params (OverlappedComponent :type Primitive%20Component%20Object%20Reference) (OtherActor :type Actor%20Object%20Reference) (OtherComp :type Primitive%20Component%20Object%20Reference) (OtherBodyIndex :type Integer))
  ;[0.3326 0.3792 1] DoorPlayerDetectionBack
  (if (== (Game|GetPlayerCharacter 0) OtherActor)
    (Variables|Default|SetPlayerBack false)
    (if (not (Variables|Default|GetDoorClosed))
      (CallFunction|ChiusuraBack))))

(event Custom|AperturaFront
  ;[1 1 1] Apertura chiusura porte col time
  (Variables|Default|SetDoorClosed false)
  (bind _aperture (Timeline|Doormoving PlayFromStart)
    (:Update
      (Transformation|SetRelativeRotation (Variables|Default|GetRotatingPoint) (Math|Rotator|MakeRotator 0.0 0.0 (Math|Float|Lerp 0.0 9e+01 _aperture)) false false))))

(event Custom|ChiusuraFront
  ;[1 1 1] Apertura chiusura porte col time
  (Variables|Default|SetDoorClosed true)
  (bind _aperture (Timeline|Doormoving ReverseFromEnd)
    (:Update
      (Transformation|SetRelativeRotation (Variables|Default|GetRotatingPoint) (Math|Rotator|MakeRotator 0.0 0.0 (Math|Float|Lerp 0.0 9e+01 _aperture)) false false))))

(event Custom|AperturaBack
  ;[1 1 1] Apertura chiusura porte col time
  (Variables|Default|SetDoorClosed false)
  (bind _aperture (Timeline|Timeline PlayFromStart)
    (:Update
      (Transformation|SetRelativeRotation (Variables|Default|GetRotatingPoint) (Math|Rotator|MakeRotator 0.0 0.0 (Math|Float|Lerp 0.0 -9e+01 _aperture)) false false))))

(event Custom|ChiusuraBack
  ;[1 1 1] Apertura chiusura porte col time
  (Variables|Default|SetDoorClosed true)
  (bind _aperture (Timeline|Timeline ReverseFromEnd)
    (:Update
      (Transformation|SetRelativeRotation (Variables|Default|GetRotatingPoint) (Math|Rotator|MakeRotator 0.0 0.0 (Math|Float|Lerp 0.0 -9e+01 _aperture)) false false))))

(event EventInteract
  ;[1 1 1] interazione per Apertura porte
  (if (Variables|Default|GetDoorClosed)
    (if (Variables|Default|GetPlayerFront)
      (if (Variables|Default|GetCanOpenFront)
        (CallFunction|AperturaFront))
      (elif (Variables|Default|GetPlayerBack)
        (if (Variables|Default|GetCanOpenBack)
          (CallFunction|AperturaBack))))))

(event EventBeginPlay
  (Variables|Default|SetDoorClosed true))

(fn ConstructionScript)